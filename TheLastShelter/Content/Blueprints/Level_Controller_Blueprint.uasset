(event EventBeginPlay)

(event Collision|EventActorBeginOverlap
  (params (OtherActor :type Actor%20Object%20Reference)))

(event EventTick
  (params (DeltaSeconds :type Float%20%28single-precision%29))
  (bind _returnvalue (Game|GetPlayerController 0))
  (bind (_worldlocation _worlddirection) (Game|Player|ConvertMouseLocationToWorldSpace _returnvalue))
  (bind _z (Math|Vector|BreakVector _worldlocation))
  (bind _z_2 (Math|Vector|BreakVector _worlddirection))
  (bind _returnvalue_2 (/ _z _z_2))
  (bind _returnvalue_3 (* _worlddirection _returnvalue_2))
  (bind _returnvalue_4 (* _returnvalue_3 -1.0))
  (bind _returnvalue_5 (+ _worldlocation _returnvalue_4))
  (bind _returnvalue_6 (+ _returnvalue_5 "0, 0,35.000000"))
  (if (Variables|Default|GetmodoConstruccion)
    (if (Variables|Default|GetsobreCasilla)
      (if (== (Variables|Default|GettipoEdificio) 3)
        (Transformation|SetActorLocation (Variables|Default|GetmodeloGenerador) (Variables|Default|GetlocationCasilla) false false)
        (else
          (Transformation|SetActorLocation (Variables|Default|GetmodeloTorreta) (Variables|Default|GetlocationCasilla) false false)))
      (elif (== (Variables|Default|GettipoEdificio) 3)
        (Transformation|SetActorLocation (Variables|Default|GetmodeloGenerador) _returnvalue_6 false false)
        (else
          (Transformation|SetActorLocation (Variables|Default|GetmodeloTorreta) _returnvalue_6 false false))))
    (elif (Variables|Default|GetmodoExplosion)
      (Transformation|SetActorLocation (Variables|Default|GetcastIndicator) _returnvalue_6 false false))))

(event Input|KeyboardEvents|Escape
  (params (Key :type Key%20Structure :default "AnyKey"))
  (:Pressed
    (CallFunction|SalirModoExplosion)
    (CallFunction|SalirModoConstruccion)))

(fn ConstructionScript
  (Variables|Default|SetrecursosActuales (Variables|Default|GetrecursosIniciales)))

(fn EntrarModoConstruccion
  (params (tipoEdificio :type Integer))
  (CallFunction|SalirModoConstruccion)
  (bind _output_get (Variables|Default|SettipoEdificio tipoEdificio))
  (Variables|Default|SetmodoConstruccion true)
  (if (== _output_get 3)
    (bind _outactors (Actor|GetAllActorsOfClass "/Game/Casilla/CasillaGenerador.CasillaGenerador_C"))
    (for _array_element _outactors
      (Rendering|SetVisibility (Variables|/Game/Casilla/CasillaGenerador.CasillaGenerador_C|GetDefaultSceneRoot _array_element) true false))
    (bind _returnvalue (Game|SpawnActorfromClass "/Game/Generador/FakeGenerador.FakeGenerador_C" (Math|Transform|MakeTransform "0, 0, 0") "Undefined" 0 0))
    (Variables|Default|SetmodeloGenerador _returnvalue)
    (else
      (bind _outactors_2 (Actor|GetAllActorsOfClass "/Game/Casilla/Casilla.Casilla_C"))
      (for _array_element_2 _outactors_2
        (Rendering|SetVisibility (Variables|/Game/Casilla/Casilla.Casilla_C|GetMalla_Casilla _array_element_2) true false))
      (if (Utilities|IsValid (Variables|Default|GetmodeloTorreta))
        (Actor|DestroyActor (Variables|Default|GetmodeloTorreta)))
      (bind _returnvalue_2 (Game|SpawnActorfromClass "/Game/Torreta/FakeTurret.FakeTurret_C" (Math|Transform|MakeTransform "0, 0, 0" "0, 0, 0" "2.000000,2.000000,2.000000") "AlwaysSpawn" 0 0))
      (Variables|Default|SetmodeloTorreta _returnvalue_2))))

(fn SalirModoConstruccion
  (bind _modelotorreta (Variables|Default|GetmodeloTorreta))
  (bind _modelogenerador (Variables|Default|GetmodeloGenerador))
  (Variables|Default|SetsobreCasilla false)
  (Variables|Default|SetmodoConstruccion false)
  (bind _outactors (Actor|GetAllActorsOfClass "/Game/Casilla/Casilla.Casilla_C"))
  (for _array_element _outactors
    (Rendering|SetVisibility (Variables|/Game/Casilla/Casilla.Casilla_C|GetMalla_Casilla _array_element) false false))
  (bind _outactors_2 (Actor|GetAllActorsOfClass "/Game/Casilla/CasillaGenerador.CasillaGenerador_C"))
  (for _array_element_2 _outactors_2
    (Rendering|SetVisibility (Variables|/Game/Casilla/CasillaGenerador.CasillaGenerador_C|GetDefaultSceneRoot _array_element_2) false false))
  (if (Utilities|IsValid _modelotorreta)
    (Actor|DestroyActor _modelotorreta))
  (if (Utilities|IsValid _modelogenerador)
    (Actor|DestroyActor _modelogenerador)))

(fn ReduceRecursos
  (params (cantidad :type Integer))
  (Variables|Default|SetrecursosActuales (- (Variables|Default|GetrecursosActuales) cantidad)))

(fn AumentaRecursos
  (params (cantidad :type Integer))
  (Variables|Default|SetrecursosActuales (+ (Variables|Default|GetrecursosActuales) cantidad)))

(fn EntrarModoExplosion
  (params (tipoExplosion :type Integer))
  (bind _radionuclear (Variables|Default|GetradioNuclear))
  (bind _radioaereo (Variables|Default|GetradioAereo))
  (bind _returnvalue (Math|Conversions|ToFloat(Integer) _radioaereo))
  (bind _returnvalue_2 (Math|Conversions|ToFloat(Integer) _radionuclear))
  (bind _returnvalue_3 (/ _returnvalue_2 3.0))
  (bind _returnvalue_4 (/ _returnvalue 3.0))
  (Variables|Default|SettipoExplosion tipoExplosion)
  (Variables|Default|SetmodoExplosion true)
  (if (== tipoExplosion 0)
    (bind _returnvalue_5 (Game|SpawnActorfromClass "/Game/HUD/cast_Material_Blueprint.cast_Material_Blueprint_C" (Math|Transform|MakeTransform "0, 0, 0" "-90.000000, 0, 0" (Math|Vector|MakeVector _returnvalue_4 _returnvalue_4 _returnvalue_4)) "Undefined" 0 0))
    (Variables|Default|SetcastIndicator _returnvalue_5)
    (elif (== tipoExplosion 1)
      (bind _returnvalue_6 (Game|SpawnActorfromClass "/Game/HUD/cast_Material_Blueprint.cast_Material_Blueprint_C" (Math|Transform|MakeTransform "0, 0, 0" "-90.000000, 0, 0" (Math|Vector|MakeVector _returnvalue_3 _returnvalue_3 _returnvalue_3)) "Undefined" 0 0))
      (Variables|Default|SetcastIndicator _returnvalue_6))))

(fn SalirModoExplosion
  (bind _castindicator (Variables|Default|GetcastIndicator))
  (bind _tipoexplosion (Variables|Default|GettipoExplosion))
  (Variables|Default|SetmodoExplosion false)
  (if (Utilities|IsValid _castindicator)
    (Actor|DestroyActor _castindicator)
    (if (== _tipoexplosion 0)
      (Variables|Default|SetcdAereo (+ (Utilities|Time|GetGameTimeinSeconds) (Variables|Default|GetcooldownAereo)))
      (elif (== _tipoexplosion 1)
        (Variables|Default|SetcdNuclear (+ (Utilities|Time|GetGameTimeinSeconds) (Variables|Default|GetcooldownNuclear)))))))

(fn ExplosionClick
  (params (Location :type Vector))
  (bind _radioaereo (Variables|Default|GetradioAereo))
  (bind _dañoaereo (Variables|Default|GetdañoAereo))
  (bind _tipoexplosion (Variables|Default|GettipoExplosion))
  (bind _radionuclear (Variables|Default|GetradioNuclear))
  (bind _dañonuclear (Variables|Default|GetdañoNuclear))
  (if (Math|Boolean|Equal(Boolean) (Variables|Default|GetmodoExplosion) true)
    (if (== _tipoexplosion 0)
      (bind _returnvalue (Effects|SpawnEmitteratLocation "/Game/StarterContent/Particles/P_Explosion.P_Explosion" Location))
      (Transformation|SetRelativeScale3D _returnvalue (Math|Vector|MakeVector (Math|Conversions|ToFloat(Integer) _radioaereo) (Math|Conversions|ToFloat(Integer) _radioaereo) (Math|Conversions|ToFloat(Integer) _radioaereo)))
      (Audio|PlaySoundatLocation "/Game/StarterContent/Audio/Explosion02.Explosion02" Location)
      (Class|GameplayStatics|ApplyRadialDamagewithFalloff (Math|Conversions|ToFloat(Integer) _dañoaereo) (* _dañoaereo 0.4) Location (* _radioaereo 0.4) (Math|Conversions|ToFloat(Integer) _radioaereo) 2.0 "/Script/Engine.DamageType" (stale _outactors) 0 0 "ECC_Visibility")
      (CallFunction|SalirModoExplosion)
      (elif (== _tipoexplosion 1)
        (bind _returnvalue_2 (Effects|SpawnEmitteratLocation "/Game/StarterContent/Particles/P_Explosion.P_Explosion" Location))
        (Transformation|SetRelativeScale3D _returnvalue_2 (Math|Vector|MakeVector (Math|Conversions|ToFloat(Integer) _radionuclear) (Math|Conversions|ToFloat(Integer) _radionuclear) (Math|Conversions|ToFloat(Integer) _radionuclear)))
        (Audio|PlaySoundatLocation "/Game/StarterContent/Audio/Explosion02.Explosion02" Location)
        (Class|GameplayStatics|ApplyRadialDamagewithFalloff (Math|Conversions|ToFloat(Integer) _dañonuclear) (* _dañonuclear 0.4) Location (* _radionuclear 0.4) (Math|Conversions|ToFloat(Integer) _radionuclear) 2.0 "/Script/Engine.DamageType" (stale _outactors) 0 0 "ECC_Visibility")
        (CallFunction|SalirModoExplosion)))))

(fn CursorEntraCasila
  (params (location :type Vector))
  (bind _modelogenerador (Variables|Default|GetmodeloGenerador))
  (bind _staticmesh (Variables|/Game/Generador/FakeGenerador.FakeGenerador_C|GetStaticMesh _modelogenerador))
  (Variables|Default|SetsobreCasilla true)
  (Variables|Default|SetlocationCasilla location)
  (if (== (Variables|Default|GettipoEdificio) 3)
    (for (_ _array_index) (Rendering|Material|GetMaterials _staticmesh)
      (Rendering|Material|SetMaterial _staticmesh _array_index "/Game/Casilla/Materials/Free/Glass/M_Glass_Blue.M_Glass_Blue"))
    (else
      (Rendering|Material|SetMaterial (Variables|/Game/Torreta/FakeTurret.FakeTurret_C|GetStaticMesh (Variables|Default|GetmodeloTorreta)) 0 "/Game/Casilla/Materials/Free/Glass/M_Glass_Blue.M_Glass_Blue"))))

(fn CursorSaleCasilla
  (bind _modelogenerador (Variables|Default|GetmodeloGenerador))
  (bind _staticmesh (Variables|/Game/Generador/FakeGenerador.FakeGenerador_C|GetStaticMesh _modelogenerador))
  (Variables|Default|SetsobreCasilla false)
  (if (== (Variables|Default|GettipoEdificio) 3)
    (for (_ _array_index) (Rendering|Material|GetMaterials _staticmesh)
      (Rendering|Material|SetMaterial _staticmesh _array_index "/Game/Casilla/Materials/Free/Glass/M_Glass_Red.M_Glass_Red"))
    (else
      (Rendering|Material|SetMaterial (Variables|/Game/Torreta/FakeTurret.FakeTurret_C|GetStaticMesh (Variables|Default|GetmodeloTorreta)) 0 "/Game/Casilla/Materials/Free/Glass/M_Glass_Red.M_Glass_Red"))))